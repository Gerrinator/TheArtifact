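; Camera Blueprint that moves its OscLightRight component and drives audio parameters from the gamepad's right stick.
; Right-stick input offsets the component on its local Y/Z plane at a fixed forward distance, and also prints the axis for testing.
; BeginPlay adds an audio component, and Tick feeds it the stick axes as JoystickX and JoystickY float parameters.
; A deprecated, sine-based mouse-position version of the movement remains disconnected.
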(event EventBeginPlay
  (bind _returnvalue (AddComponent|AddAudioComponent false)))

(event Collision|EventActorBeginOverlap
  (params (OtherActor :type Actor%20Object%20Reference)))

(event EventTick
  (params (DeltaSeconds :type Float%20%28single-precision%29))
  (Audio|Parameter|SetFloatParameter (stale EventBeginPlay _returnvalue) "JoystickY" (.Y (Math|Vector|BreakVector (stale Input|GamepadEvents|GamepadRight2D AxisValue))) :!class /Script/AudioExtensions.AudioParameterControllerInterface)
  (Audio|Parameter|SetFloatParameter (stale EventBeginPlay _returnvalue) "JoystickX" (.X (Math|Vector|BreakVector (stale Input|GamepadEvents|GamepadRight2D AxisValue))) :!class /Script/AudioExtensions.AudioParameterControllerInterface))

(event Input|GamepadEvents|GamepadDPadUp
  (params (Key :type Key%20Structure :default "None"))
  ;[1 1 1] For use with mouse movement (deprecated)
)

(event Input|KeyboardEvents|AnyKey
  (params (Key :type Key%20Structure :default "None"))
  ;[0 0 0] For testing controller input
)

(event Input|GamepadEvents|GamepadRight2D
  (params (AxisValue :type Vector :default "0, 0, 0"))
  ;[0 0 0] For testing controller input
  (Development|PrintString (Utilities|String|ToString(Vector) AxisValue)))

(event Input|GamepadEvents|GamepadRight2D
  (params (AxisValue :type Vector :default "0, 0, 0"))
  (bind (_x _y) (Math|Vector|BreakVector AxisValue))
  (Transformation|SetRelativeLocation (Variables|Default|GetOscLightRight) (Math|Vector|MakeVector 178.0 (* _x 5e+01) (* _y -5e+01)) false false))

(fn ConstructionScript)